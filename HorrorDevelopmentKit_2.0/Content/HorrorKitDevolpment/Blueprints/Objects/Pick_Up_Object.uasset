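; Pickup actor for the horror kit that adds its item to the player's inventory when interacted with.
; Interaction walks a nested chain of nine slot-filled flags on the main character through CheckInventorySlot.
; The first passing slot receives the name, mesh, image and description in ItemList, then the flag is set and the actor destroys itself.
; A DoOnce with a delayed reset throttles repeat interaction, and construction applies the configured mesh.
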(event `self.ReceiveBeginPlay`
  (bind _asmain_character_blueprint (cast `/Game/HorrorKitDevolpment/Blueprints/Character/Main_Character_Blueprint` (`GameplayStatics.GetPlayerCharacter` 0)))
  (set `self.Main_Character` _asmain_character_blueprint))

(event `/Game/HorrorKitDevolpment/Blueprints/Character/Lists/Interact.Interactable Object`
  (`/Engine/EditorBlueprintResources/StandardMacros.DoOnce` false :!label _label
    (:`Completed`
      (if (`self.Check Inventory Slot` (`/Game/HorrorKitDevolpment/Blueprints/Character/Main_Character_Blueprint.Inventory 1 Filled` (`self.Main_Character`)))
        (`self.Add Item to Inventory` 0)
        (set `/Game/HorrorKitDevolpment/Blueprints/Character/Main_Character_Blueprint.Inventory 1 Filled` true (`self.Main_Character`))
        (`self.K2_DestroyActor`)
        (elif (`self.Check Inventory Slot` (`/Game/HorrorKitDevolpment/Blueprints/Character/Main_Character_Blueprint.Inventory 2 Filled` (`self.Main_Character`)))
          (`self.Add Item to Inventory` 1)
          (set `/Game/HorrorKitDevolpment/Blueprints/Character/Main_Character_Blueprint.Inventory 2 Filled` true (`self.Main_Character`))
          (`self.K2_DestroyActor`)
          (elif (`self.Check Inventory Slot` (`/Game/HorrorKitDevolpment/Blueprints/Character/Main_Character_Blueprint.Inventory 3 Filled` (`self.Main_Character`)))
            (`self.Add Item to Inventory` 2)
            (set `/Game/HorrorKitDevolpment/Blueprints/Character/Main_Character_Blueprint.Inventory 3 Filled` true (`self.Main_Character`))
            (`self.K2_DestroyActor`)
            (elif (`self.Check Inventory Slot` (`/Game/HorrorKitDevolpment/Blueprints/Character/Main_Character_Blueprint.Inventory 4 Filled` (`self.Main_Character`)))
              (`self.Add Item to Inventory` 3)
              (set `/Game/HorrorKitDevolpment/Blueprints/Character/Main_Character_Blueprint.Inventory 4 Filled` true (`self.Main_Character`))
              (`self.K2_DestroyActor`)
              (elif (`self.Check Inventory Slot` (`/Game/HorrorKitDevolpment/Blueprints/Character/Main_Character_Blueprint.Inventory 5 Filled` (`self.Main_Character`)))
                (`self.Add Item to Inventory` 4)
                (set `/Game/HorrorKitDevolpment/Blueprints/Character/Main_Character_Blueprint.Inventory 5 Filled` true (`self.Main_Character`))
                (`self.K2_DestroyActor`)
                (elif (`self.Check Inventory Slot` (`/Game/HorrorKitDevolpment/Blueprints/Character/Main_Character_Blueprint.Inventory 6 Filled` (`self.Main_Character`)))
                  (`self.Add Item to Inventory` 5)
                  (set `/Game/HorrorKitDevolpment/Blueprints/Character/Main_Character_Blueprint.Inventory 6 Filled` true (`self.Main_Character`))
                  (`self.K2_DestroyActor`)
                  (elif (`self.Check Inventory Slot` (`/Game/HorrorKitDevolpment/Blueprints/Character/Main_Character_Blueprint.Inventory 7 Filled` (`self.Main_Character`)))
                    (`self.Add Item to Inventory` 6)
                    (set `/Game/HorrorKitDevolpment/Blueprints/Character/Main_Character_Blueprint.Inventory 7 Filled` true (`self.Main_Character`))
                    (`self.K2_DestroyActor`)
                    (elif (`self.Check Inventory Slot` (`/Game/HorrorKitDevolpment/Blueprints/Character/Main_Character_Blueprint.Inventory 8 Filled` (`self.Main_Character`)))
                      (`self.Add Item to Inventory` 7)
                      (set `/Game/HorrorKitDevolpment/Blueprints/Character/Main_Character_Blueprint.Inventory 8 Filled` true (`self.Main_Character`))
                      (`self.K2_DestroyActor`)
                      (elif (`self.Check Inventory Slot` (`/Game/HorrorKitDevolpment/Blueprints/Character/Main_Character_Blueprint.Inventory 9 Filled` (`self.Main_Character`)))
                        (`self.Add Item to Inventory` 8)
                        (set `/Game/HorrorKitDevolpment/Blueprints/Character/Main_Character_Blueprint.Inventory 9 Filled` true (`self.Main_Character`))
                        (`self.K2_DestroyActor`))))))))))
      (`KismetSystemLibrary.Delay` 1.0)
      (`self.Reset`))))

(event `Reset`
  (goto _label :!via `Reset`))

(fn `Add Item to Inventory`
  (params (`Inventory Slot` :type Integer))
  (bind _main_character (`self.Main_Character`))
  (`KismetArrayLibrary.Array_Insert` (`/Game/HorrorKitDevolpment/Blueprints/Character/Main_Character_Blueprint.Item List ` (`self.Main_Character`)) (make `/Game/HorrorKitDevolpment/Blueprints/Character/Item_Varaibles` (`self.Name Of Object`) (`StaticMeshComponent.StaticMesh` (`self.StaticMesh`)) (`self.Image`) (`self.Item Description`)) `Inventory Slot`)
  (set `/Game/HorrorKitDevolpment/Blueprints/Character/Main_Character_Blueprint.Inventory Slots` (+ (`/Game/HorrorKitDevolpment/Blueprints/Character/Main_Character_Blueprint.Inventory Slots` _main_character) 1) _main_character)
  (return))

(fn `UserConstructionScript`
  (`StaticMeshComponent.SetStaticMesh` (`self.StaticMesh`) (`self.Mesh`)))